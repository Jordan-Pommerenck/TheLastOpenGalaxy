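; Helper actor that drives hyperspace jumps for its instigator base_ship, on timed arrival or after the last waypoint of a non-looping route.
; On BeginPlay it samples HyperCurve into forward and reversed distance-factor arrays, and hides ships awaiting delayed arrival.
; Looping timers step the ship along its forward vector through both arrays, switching by distance from InitialLocation.
; The jump ends with a pitch-scaled shockwave sound, then the handler destroys itself.
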(event `initialize_hyper_curve_data`
  (bind _hypercurve (`self.HyperCurve`))
  (bind (_mintime _maxtime) (`CurveBase.GetTimeRange` _hypercurve))
  (bind _output_get (set `self.initial_location` (+ (* (`KismetMathLibrary.NegateVector` (`self.GetActorForwardVector` (`self.base_ship`))) (`KismetMathLibrary.Conv_DoubleToVector` (`self.FinalDistance [km]`))) (`self.final_location`))))
  (`self.K2_SetActorLocation` _output_get false true)
  (for _index (range 501)
    (bind _returnvalue (/ (* _index _maxtime) 500.0))
    (`KismetArrayLibrary.Array_Add` (`self.HyperTimes`) _returnvalue)
    (`KismetArrayLibrary.Array_Add` (`self.HyperDistanceFactors`) (/ (`CurveFloat.GetFloatValue` _hypercurve _returnvalue) (`KismetMathLibrary.FMax` _returnvalue 1e-06))))
  (bind (_arrayindex _arrayelement) (`/Engine/EditorBlueprintResources/StandardMacros.ReverseForEachLoop` (`self.HyperDistanceFactors`))
    (:`LoopBody`
      (`KismetArrayLibrary.Array_Add` (`self.HyperDistanceFactorReverse`) _arrayelement))
    (:`Completed`
      (set `self.HyperTimeCounter` (/ _maxtime 500.0)))))

(event `initialize_base_parameters`
  (bind _asbase_ship (cast `/Game/Blueprints/base_ship` (`self.Instigator`)))
  (bind _output_get (set `self.base_ship` _asbase_ship))
  (bind _asaicontroller (cast `AIController` (`Pawn.GetController` _output_get)))
  (set `self.AI_controller` _asaicontroller)
  (set `self.FinalDistance [km]` (`self.convert_to_km` 2.0 (`/Game/Blueprints/base_ship.scale_factor` _output_get)))
  (`self.initialize_hyper_curve_data`))

(event `self.ReceiveBeginPlay`
  (bind (_names _ship_type _center_location _center_rotation _difficulty_level _team _formation_shape _ai_capital_behavior _i_need_to_escort _i_need_escorted _i_need_disabled _waypoint_looping _waypoints _hyper_in_time) (break `/Game/Data/Structures/spawn_variables` (`self.base_ship_struct`)))
  (`self.initialize_base_parameters`)
  (`KismetSystemLibrary.Delay` 0.1)
  (set `self.final_location` _center_location)
  ;[1 1 1] need to hyper in
  (bind _output_get (set `self.hyper_in_time` _hyper_in_time))
  (`|ExecutionSequence`
    (:`then_0`
      (if (> _output_get 0)
        (`KismetSystemLibrary.K2_SetTimerDelegate` (`|CreateDelegate` :!event `hpyer_in`) (`KismetMathLibrary.Conv_IntToDouble` _output_get))
        ;[1 1 1] Hide the actor until ready
        (`self.SetActorHiddenInGame` (`self.base_ship`) true)))
    (:`then_1`
      (if (and (not _waypoint_looping) (> (`KismetArrayLibrary.Array_Length` _waypoints) 0))
        (bind _returnvalue (`KismetSystemLibrary.K2_SetTimerDelegate` (`|CreateDelegate` :!event `reached_waypoint_final`) 0.2 true))
        (set `self.reached_waypoint_timer` _returnvalue)))))

(event `hpyer_in`
  (`self.SetActorHiddenInGame` (`self.base_ship`) false)
  (bind _returnvalue (`KismetSystemLibrary.K2_SetTimerDelegate` (`|CreateDelegate` :!event `HYPERING`) (`self.HyperTimeCounter`) true :!label _label))
  (set `self.hypering_timer` _returnvalue))

(event `reached_waypoint_final`
  (bind _base_ship (`self.base_ship`))
  (bind _waypoints (`master_ship.waypoints` _base_ship))
  (if (== (`self.K2_GetActorLocation` _base_ship) (`|GetArrayItem` _waypoints (`KismetArrayLibrary.Array_LastIndex` _waypoints)))
    (`KismetSystemLibrary.K2_ClearAndInvalidateTimerHandle` (`self.reached_waypoint_timer`))
    (goto _label)))

(event `HYPERING`
  (bind _base_ship (`self.base_ship`))
  (bind _counter (`self.Counter`))
  (bind _hyperdistancefactors (`self.HyperDistanceFactors`))
  (bind _returnvalue (- (`KismetArrayLibrary.Array_Length` _hyperdistancefactors) 1))
  (bind _returnvalue_2 (< _counter _returnvalue))
  (`self.K2_SetActorLocation` _base_ship (`self.HyperspaceMath` _base_ship (`|GetArrayItem` _hyperdistancefactors _counter) (`self.FinalDistance [km]`)) false false)
  (if (> (`KismetMathLibrary.VSize` (- (`self.initial_location`) (`self.K2_GetActorLocation` (`self.base_ship`)))) (* (`self.FinalDistance [km]`) 0.5))
    (if _returnvalue_2
      (`/Engine/EditorBlueprintResources/StandardMacros.IncrementInt` _counter)
      (else
        (set `self.Counter` _returnvalue)))
    (else
      (set `self.Counter` (select `bool` _returnvalue_2 :`true` (- _returnvalue (`self.Counter`))))
      (`KismetSystemLibrary.K2_ClearAndInvalidateTimerHandle` (`self.hypering_timer`))
      (bind _returnvalue_3 (`KismetSystemLibrary.K2_SetTimerDelegate` (delegate `CustomEvent_0`) (`self.HyperTimeCounter`) true))
      (set `self.NewVar_1` _returnvalue_3))))

(event `CustomEvent_0`
  (bind _base_ship (`self.base_ship`))
  (bind _hyperdistancefactorreverse (`self.HyperDistanceFactorReverse`))
  (bind _base_ship_2 (`self.base_ship`))
  (bind _counter (`self.Counter`))
  (bind _returnvalue (`self.K2_GetActorLocation` _base_ship))
  (`self.K2_SetActorLocation` _base_ship_2 (`self.HyperspaceMath` _base_ship_2 (`|GetArrayItem` _hyperdistancefactorreverse _counter) (`self.FinalDistance [km]`)) false false)
  (if (< (`KismetMathLibrary.VSize` (- (`self.initial_location`) _returnvalue)) (`self.FinalDistance [km]`))
    (if (< _counter (- (`KismetArrayLibrary.Array_Length` _hyperdistancefactorreverse) 1))
      (`/Engine/EditorBlueprintResources/StandardMacros.IncrementInt` _counter)
      (else
        (`KismetSystemLibrary.K2_ClearAndInvalidateTimerHandle` (`self.NewVar_1`) :!label _label_2)
        ;[1 1 1] Sound
        (`GameplayStatics.PlaySoundAtLocation` "/Game/Audio/HyperInShockWave.HyperInShockWave" _returnvalue (struct) 100.0 (`KismetMathLibrary.FClamp` (`KismetMathLibrary.Loge` (`KismetMathLibrary.Abs` (/ (- (`KismetMathLibrary.GetMaxElement` (`self.final_location`)) (`self.FinalDistance [km]`)) (* 1.0 (`/Game/Blueprints/base_ship.scale_factor` _base_ship) 1000.0)))) 0.5 3.0) 0.0 "/Game/Audio/Attenuation_HyperWave.Attenuation_HyperWave" "/Game/Audio/Concurrency_HyperWave.Concurrency_HyperWave" _base_ship)
        (`KismetSystemLibrary.Delay` 2.0)
        (`self.K2_DestroyActor`)))
    (else
      (goto _label_2))))

(fn `convert_to_km`
  (params (number_km :type "Float (double-precision)") (scale_factor :type "Float (double-precision)"))
  (returns (ReturnValue :type "Float (double-precision)"))
  (return (* number_km scale_factor 1000.0)))

(fn `HyperspaceMath`
  (params (BaseShip :type "Actor Object Reference") (TimelineFactor :type "Float (double-precision)") (FinalDistance :type "Float (double-precision)"))
  (returns (ReturnValue :type "Vector Structure"))
  (return (+ (* (`self.GetActorForwardVector` BaseShip) (`KismetMathLibrary.Conv_DoubleToVector` (* TimelineFactor 1.0 FinalDistance))) (`self.K2_GetActorLocation` BaseShip))))

(fn `UserConstructionScript`)