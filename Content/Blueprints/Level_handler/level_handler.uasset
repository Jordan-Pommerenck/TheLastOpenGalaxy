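; Level handler Blueprint that drafts loading a level from data and spawning its AI ships; none of its logic is connected to an event.
; One fragment reads a JSON file into a data table and takes the first row as LevelData.
; Others open or stream the named level, or spawn counted AI ships from AllSpawnCraft with a fighter behavior tree, team and difficulty.
; The file path is empty and the construction script does nothing.
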(fn `UserConstructionScript`)