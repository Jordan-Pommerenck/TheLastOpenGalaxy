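; Ship combat game mode that decides win or loss for Dogfight, Escort and Disable levels.
; After BeginPlay it sorts ships by team and derives targets from the game instance's LevelData fractions.
; Looping timers poll player survival and kills, escapes beyond a scaled distance from origin, or disabled ships, rescaling the AI check interval near thresholds.
; Outcomes set WinOrLose on the game instance, then open the victory condition level.
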(event `Human Actor Check`
  ;[0.25 0.25 0.25] Check for wether Human Player is alive
  (`/Engine/EditorBlueprintResources/StandardMacros.IsValid` (`Controller.K2_GetPawn` (`GameplayStatics.GetPlayerController` 0))
    (:`Is Not Valid`
      (set `/Game/Blueprints/GameInstance/game_info_instance.win_or_lose` false (`self.game_inst_ref`))
      (`WidgetLayoutLibrary.RemoveAllWidgets`)
      (`self.victory_screen`))))

(event `victory_screen`
  ;[0.25 0.25 0.25] Go to victory condition level with either win or lose set (so we know what to display)
  (`KismetSystemLibrary.Delay` 0.05)
  (`GameplayStatics.OpenLevel` (`self.victory_condition_level`)))

(event `self.ReceiveBeginPlay`
  ;[0 0 0] Starting ship is deleted
  (`KismetSystemLibrary.Delay` 1.0)
  (bind _asgame_info_instance (cast `/Game/Blueprints/GameInstance/game_info_instance` (`GameplayStatics.GetGameInstance`)))
  (set `self.game_inst_ref` _asgame_info_instance)
  (bind _asbase_ship (cast `/Game/Blueprints/base_ship` (`Controller.K2_GetPawn` (`GameplayStatics.GetPlayerController` 0))))
  (set `self.base_ship` _asbase_ship)
  (`self.game_mode_setup`))

(event `game_mode_setup`
  (bind _ai_time_check (`self.AI_time_check`))
  (switch `/Game/Blueprints/GameMode/game_mode_type` (`.game_mode_39_AF4434614C5D84F63977C3B275028A2D` (break `/Game/Data/Structures/spawn_creation` (`/Game/Blueprints/GameInstance/game_info_instance.level_data` (`self.game_inst_ref`))))
    (:`NewEnumerator0`
      (`self.dogfight_find_all_ships`)
      (bind _returnvalue (`KismetSystemLibrary.K2_SetTimerDelegate` (`|CreateDelegate` :!event `dogfight_AI_actor_check`) _ai_time_check true))
      (set `self.AI_dogfight_check_timer` _returnvalue))
    (:`NewEnumerator1`
      (`self.escort_find_all_ships`)
      (bind _returnvalue_2 (`KismetSystemLibrary.K2_SetTimerDelegate` (`|CreateDelegate` :!event `escort_AI_actor_check`) _ai_time_check true))
      (set `self.AI_escort_check_timer` _returnvalue_2))
    (:`NewEnumerator2`
      (`self.disable_find_all_ships`)
      (bind _returnvalue_3 (`KismetSystemLibrary.K2_SetTimerDelegate` (`|CreateDelegate` :!event `disable_AI_actor_check`) _ai_time_check true))
      (set `self.AI_disable_check_timer` _returnvalue_3)))
  (`KismetSystemLibrary.K2_SetTimerDelegate` (`|CreateDelegate` :!event `Human Actor Check`) (`self.human_time_check`) true))

(event `dogfight_find_all_ships`
  (bind _base_ship (`self.base_ship`))
  (bind _returnvalue (`KismetArrayLibrary.Array_Length` (`self.all_enemies`)))
  (bind _returnvalue_2 (`KismetArrayLibrary.Array_Length` (`self.all_allies`)))
  (bind _outactors (`GameplayStatics.GetAllActorsOfClass` "/Game/Blueprints/base_ship.base_ship_C"))
  (for _array_element _outactors
    (`/Engine/EditorBlueprintResources/StandardMacros.IsValid` _base_ship
      (:`Is Valid`
        (`/Engine/EditorBlueprintResources/StandardMacros.IsValid` _array_element
          (:`Is Valid`
            (if (`|EnumInequality` (`master_ship.my_team` _array_element) (`master_ship.my_team` _base_ship))
              (`KismetArrayLibrary.Array_Add` (`self.all_enemies`) _array_element)
              (`KismetArrayLibrary.Array_Add` (`self.all_game_mode_menu_enemies`) _array_element)
              (else
                (`KismetArrayLibrary.Array_Add` (`self.all_allies`) _array_element)
                (`KismetArrayLibrary.Array_Add` (`self.all_game_mode_menu_allies`) _array_element))))))))
  (set `self.initial_ally_count` (`KismetMathLibrary.Clamp` (`KismetMathLibrary.Round` (* _returnvalue_2 (- 1.0 (`.dogfight_ally_frac_destroy_57_02FF5D7847C9B5F942AE0D818B9495B8` (break `/Game/Data/Structures/spawn_creation` (`/Game/Blueprints/GameInstance/game_info_instance.level_data` (`self.game_inst_ref`))))))) 0 (- _returnvalue_2 1)))
  (set `self.initial_enemy_count` (`KismetMathLibrary.Clamp` (`KismetMathLibrary.Round` (* _returnvalue (- 1.0 (`.dogfight_enemy_frac_destroy_56_698918C04173F207FE31C19FF7CABBC5` (break `/Game/Data/Structures/spawn_creation` (`/Game/Blueprints/GameInstance/game_info_instance.level_data` (`self.game_inst_ref`))))))) 0 (- _returnvalue 1)))
  (set `self.init_dogfight_num_enemies` _returnvalue)
  (set `self.init_dogfight_num_allies` _returnvalue_2))

(event `escort_find_all_ships`
  (bind _base_ship (`self.base_ship`))
  (bind _all_allies (`self.all_allies`))
  (bind (_init_count _arrray_length) (`self.init_count` _all_allies (`.escort_ally_frac_destroy_58_CB2B490149B9A6CC97AB04BED0F80B14` (break `/Game/Data/Structures/spawn_creation` (`/Game/Blueprints/GameInstance/game_info_instance.level_data` (`self.game_inst_ref`))))))
  (bind (_init_count_2 _arrray_length_2) (`self.init_count` (`self.all_enemies`) (`.escort_enemy_frac_destroy_60_BB18EE0C455298C65D18C9A87DE73443` (break `/Game/Data/Structures/spawn_creation` (`/Game/Blueprints/GameInstance/game_info_instance.level_data` (`self.game_inst_ref`))))))
  (bind _outactors (`GameplayStatics.GetAllActorsOfClass` "/Game/Blueprints/base_ship.base_ship_C"))
  (for _array_element _outactors
    (`/Engine/EditorBlueprintResources/StandardMacros.IsValid` _base_ship
      (:`Is Valid`
        (`/Engine/EditorBlueprintResources/StandardMacros.IsValid` _array_element
          (:`Is Valid`
            (if (`master_ship.i_need_escorting` _array_element)
              (bind _returnvalue (`|EnumInequality` (`master_ship.my_team` _array_element) (`master_ship.my_team` _base_ship)))
              (if _returnvalue
                (`KismetArrayLibrary.Array_Add` (`self.all_enemies`) _array_element)
                (`KismetArrayLibrary.Array_Add` (`self.all_game_mode_menu_enemies`) _array_element :!label _label)
                (else
                  (`KismetArrayLibrary.Array_Add` (`self.all_allies`) _array_element)
                  (`KismetArrayLibrary.Array_Add` (`self.all_game_mode_menu_allies`) _array_element :!label _label_2)))
              (elif _returnvalue
                (goto _label)
                (else
                  (goto _label_2)))))))))
  (set `self.num_ally_get_away` _init_count)
  (set `self.initial_ally_count` _arrray_length)
  (set `self.num_enemy_get_away` _init_count_2)
  (set `self.initial_enemy_count` _arrray_length_2)
  (set `self.dont_check_allies` (== (`KismetArrayLibrary.Array_Length` _all_allies) 0)))

(event `disable_find_all_ships`
  (bind _base_ship (`self.base_ship`))
  (bind _all_allies (`self.all_allies`))
  (bind _all_enemies (`self.all_enemies`))
  (bind (_init_count _arrray_length) (`self.init_count` _all_allies (`.disable_ally_frac_destroy_64_1E39EF49463FB917E48586BDED9C03E3` (break `/Game/Data/Structures/spawn_creation` (`/Game/Blueprints/GameInstance/game_info_instance.level_data` (`self.game_inst_ref`))))))
  (bind (_init_count_2 _arrray_length_2) (`self.init_count` _all_enemies (`.disable_enemy_frac_destroy_63_F4F6E0BB40A381131F2B16BAFED25714` (break `/Game/Data/Structures/spawn_creation` (`/Game/Blueprints/GameInstance/game_info_instance.level_data` (`self.game_inst_ref`))))))
  (bind _outactors (`GameplayStatics.GetAllActorsOfClass` "/Game/Blueprints/base_ship.base_ship_C"))
  (for _array_element _outactors
    (`/Engine/EditorBlueprintResources/StandardMacros.IsValid` _base_ship
      (:`Is Valid`
        (`/Engine/EditorBlueprintResources/StandardMacros.IsValid` _array_element
          (:`Is Valid`
            (if (`master_ship.i_need_disabled` _array_element)
              (bind _returnvalue (`|EnumInequality` (`master_ship.my_team` _array_element) (`master_ship.my_team` _base_ship)))
              (if _returnvalue
                (`KismetArrayLibrary.Array_Add` (`self.all_enemies`) _array_element)
                (`KismetArrayLibrary.Array_Add` (`self.all_game_mode_menu_enemies`) _array_element :!label _label_3)
                (else
                  (`KismetArrayLibrary.Array_Add` (`self.all_allies`) _array_element)
                  (`KismetArrayLibrary.Array_Add` (`self.all_game_mode_menu_allies`) _array_element :!label _label_4)))
              (elif _returnvalue
                (goto _label_3)
                (else
                  (goto _label_4)))))))))
  (set `self.num_ally_disabled` _init_count)
  (set `self.initial_ally_count` _arrray_length)
  (set `self.num_enemy_disabled` _init_count_2)
  (set `self.initial_enemy_count` _arrray_length_2)
  (set `self.dont_check_allies` (== (`KismetArrayLibrary.Array_Length` _all_allies) 0))
  (set `self.dont_check_enemies` (== (`KismetArrayLibrary.Array_Length` _all_enemies) 0)))

(event `dogfight_AI_actor_check`
  (bind _all_enemies (`self.all_enemies`))
  (bind _all_allies (`self.all_allies`))
  ;[1 1 1] Dogfight code
  (bind (_arrayindex _arrayelement) (`/Engine/EditorBlueprintResources/StandardMacros.ReverseForEachLoop` _all_enemies)
    (:`LoopBody`
      (`self.dogfight_remove_enemy_index` _arrayelement _arrayindex))
    (:`Completed`
      (bind (_arrayindex_2 _arrayelement_2) (`/Engine/EditorBlueprintResources/StandardMacros.ReverseForEachLoop` _all_allies)
        (:`LoopBody`
          (`self.dogfight_remove_ally_index` _arrayelement_2 _arrayindex_2))
        (:`Completed`
          (`self.enemy_frac_check`)
          (`self.ally_frac_check`)
          (if (or (`KismetMathLibrary.NearlyEqual_FloatFloat` (`KismetMathLibrary.Conv_IntToDouble` (`KismetArrayLibrary.Array_Length` _all_enemies)) (`KismetMathLibrary.Conv_IntToDouble` (`self.initial_enemy_count`)) 2.0) (`KismetMathLibrary.NearlyEqual_FloatFloat` (`KismetMathLibrary.Conv_IntToDouble` (`KismetArrayLibrary.Array_Length` _all_allies)) (`KismetMathLibrary.Conv_IntToDouble` (`self.initial_enemy_count`)) 2.0))
            (`/Engine/EditorBlueprintResources/StandardMacros.DoOnce` false
              (:`Completed`
                (`KismetSystemLibrary.K2_ClearAndInvalidateTimerHandle` (`self.AI_dogfight_check_timer`))
                (`KismetSystemLibrary.K2_SetTimerDelegate` (`|CreateDelegate` :!event `dogfight_AI_actor_check`) (* (`self.AI_time_check`) (`self.time_reduce_factor`)) true)))))))))

(event `enemy_frac_check`
  ;[1 1 1] Dogfight code
  (if (<= (`KismetArrayLibrary.Array_Length` (`self.all_enemies`)) (`self.initial_enemy_count`))
    (set `/Game/Blueprints/GameInstance/game_info_instance.win_or_lose` true (`self.game_inst_ref`))
    (`self.victory_screen`)))

(event `ally_frac_check`
  ;[1 1 1] Dogfight code
  (if (<= (`KismetArrayLibrary.Array_Length` (`self.all_allies`)) (`self.initial_ally_count`))
    (set `/Game/Blueprints/GameInstance/game_info_instance.win_or_lose` false (`self.game_inst_ref`))
    (`self.victory_screen`)))

(event `dogfight_remove_enemy_index`
  (params (InputObject :type "Object Object Reference") (index_to_remove :type Integer))
  ;[1 1 1] Dogfight code
  (`/Engine/EditorBlueprintResources/StandardMacros.IsValid` InputObject
    (:`Is Not Valid`
      (`KismetArrayLibrary.Array_Remove` (`self.all_enemies`) index_to_remove))))

(event `dogfight_remove_ally_index`
  (params (InputObject :type "Object Object Reference") (index_to_remove :type Integer))
  ;[1 1 1] Dogfight code
  (`/Engine/EditorBlueprintResources/StandardMacros.IsValid` InputObject
    (:`Is Not Valid`
      (`KismetArrayLibrary.Array_Remove` (`self.all_allies`) index_to_remove))))

(event `disable_AI_actor_check`
  (bind _all_enemies (`self.all_enemies`))
  (bind _all_allies (`self.all_allies`))
  ;[1 1 1] Disable code
  (bind (_arrayindex _arrayelement) (`/Engine/EditorBlueprintResources/StandardMacros.ReverseForEachLoop` _all_enemies)
    (:`LoopBody`
      (`self.disable_remove_enemy` _arrayelement))
    (:`Completed`
      (bind (_arrayindex_2 _arrayelement_2) (`/Engine/EditorBlueprintResources/StandardMacros.ReverseForEachLoop` _all_allies)
        (:`LoopBody`
          (`self.disable_remove_ally` _arrayelement_2))
        (:`Completed`
          (`self.enemy_disable_frac`)
          (`self.ally_disable_frac`)
          (`self.destroy_all_enemies`)
          (if (or (`KismetMathLibrary.NearlyEqual_FloatFloat` (`KismetMathLibrary.Conv_IntToDouble` (`KismetArrayLibrary.Array_Length` _all_enemies)) (`KismetMathLibrary.Conv_IntToDouble` (`self.num_ally_disabled`)) 2.0) (`KismetMathLibrary.NearlyEqual_FloatFloat` (`KismetMathLibrary.Conv_IntToDouble` (`KismetArrayLibrary.Array_Length` _all_allies)) (`KismetMathLibrary.Conv_IntToDouble` (`self.num_enemy_disabled`)) 2.0))
            (`/Engine/EditorBlueprintResources/StandardMacros.DoOnce` false
              (:`Completed`
                (`KismetSystemLibrary.K2_ClearAndInvalidateTimerHandle` (`self.AI_disable_check_timer`))
                (`KismetSystemLibrary.K2_SetTimerDelegate` (`|CreateDelegate` :!event `disable_AI_actor_check`) (* (`self.AI_time_check`) (`self.time_reduce_factor`)) true)))))))))

(event `enemy_disable_frac`
  ;[1 1 1] Disable code
  (if (not (`self.dont_check_enemies`))
    (set `self.enemy_got_disabled` (`KismetMathLibrary.Clamp` (`self.enemy_got_disabled`) 0 (`self.num_enemy_disabled`)))
    (if (>= (`self.enemy_got_disabled`) (`self.num_enemy_disabled`))
      (set `/Game/Blueprints/GameInstance/game_info_instance.win_or_lose` true (`self.game_inst_ref`) :!label _label_5)
      (`self.victory_screen`))))

(event `destroy_all_enemies`
  ;[1 1 1] Disable code
  (if (== (`KismetArrayLibrary.Array_Length` (`self.all_game_mode_menu_enemies`)) 0)
    (goto _label_5)))

(event `ally_disable_frac`
  ;[1 1 1] Disable code
  (if (not (`self.dont_check_allies`))
    (set `self.ally_got_disabled` (`KismetMathLibrary.Clamp` (`self.ally_got_disabled`) 0 (`self.num_ally_disabled`)))
    (if (>= (`self.ally_got_disabled`) (`self.num_ally_disabled`))
      (set `/Game/Blueprints/GameInstance/game_info_instance.win_or_lose` false (`self.game_inst_ref`))
      (`self.victory_screen`))))

(event `disable_remove_enemy`
  (params (InputObject :type "/Game/Blueprints/base_ship Object Reference"))
  (bind _enemy_got_disabled (`self.enemy_got_disabled`))
  ;[1 1 1] Disable code
  (`/Engine/EditorBlueprintResources/StandardMacros.IsValid` InputObject
    (:`Is Valid`
      (if (`master_ship.i_am_disabled` InputObject)
        (`/Engine/EditorBlueprintResources/StandardMacros.IncrementInt` _enemy_got_disabled)
        (else
          (`/Engine/EditorBlueprintResources/StandardMacros.DecrementInt` _enemy_got_disabled))))
    (:`Is Not Valid`
      (set `/Game/Blueprints/GameInstance/game_info_instance.win_or_lose` false (`self.game_inst_ref`) :!label _label_6)
      (`self.victory_screen`))))

(event `disable_remove_ally`
  (params (InputObject :type "/Game/Blueprints/base_ship Object Reference"))
  (bind _ally_got_disabled (`self.ally_got_disabled`))
  ;[1 1 1] Disable code
  (`/Engine/EditorBlueprintResources/StandardMacros.IsValid` InputObject
    (:`Is Valid`
      (if (`master_ship.i_am_disabled` InputObject)
        (`/Engine/EditorBlueprintResources/StandardMacros.IncrementInt` _ally_got_disabled)
        (else
          (`/Engine/EditorBlueprintResources/StandardMacros.DecrementInt` _ally_got_disabled))))
    (:`Is Not Valid`
      (goto _label_6))))

(event `escort_AI_actor_check`
  (bind _all_allies (`self.all_allies`))
  (bind _all_enemies (`self.all_enemies`))
  ;[1 1 1] Escort code
  (bind (_arrayindex _arrayelement) (`/Engine/EditorBlueprintResources/StandardMacros.ReverseForEachLoop` _all_enemies)
    (:`LoopBody`
      (`self.escort_remove_enemy` _arrayelement))
    (:`Completed`
      (bind (_arrayindex_2 _arrayelement_2) (`/Engine/EditorBlueprintResources/StandardMacros.ReverseForEachLoop` _all_allies)
        (:`LoopBody`
          (`self.escort_remove_ally` _arrayelement_2))
        (:`Completed`
          (`self.enemy_escort_frac`)
          (`self.ally_escort_frac`)
          (`KismetSystemLibrary.Delay` 0.2)
          (`self.escort_check_alive`)
          (if (or (`KismetMathLibrary.NearlyEqual_FloatFloat` (`KismetMathLibrary.Conv_IntToDouble` (`KismetArrayLibrary.Array_Length` _all_enemies)) (`KismetMathLibrary.Conv_IntToDouble` (`self.num_enemy_get_away`)) 2.0) (and (`KismetMathLibrary.NearlyEqual_FloatFloat` (`KismetMathLibrary.Conv_IntToDouble` (`KismetArrayLibrary.Array_Length` _all_allies)) (`KismetMathLibrary.Conv_IntToDouble` (`self.num_ally_get_away`)) 2.0) (not (`self.dont_check_allies`))))
            (`/Engine/EditorBlueprintResources/StandardMacros.DoOnce` false
              (:`Completed`
                (`KismetSystemLibrary.K2_ClearAndInvalidateTimerHandle` (`self.AI_escort_check_timer`))
                (`KismetSystemLibrary.K2_SetTimerDelegate` (`|CreateDelegate` :!event `escort_AI_actor_check`) (* (`self.AI_time_check`) (`self.time_reduce_factor`)) true)))))))))

(event `enemy_escort_frac`
  ;[1 1 1] Escort code
  (if (>= (`self.enemy_got_away`) (`self.num_enemy_get_away`))
    (set `/Game/Blueprints/GameInstance/game_info_instance.win_or_lose` false (`self.game_inst_ref`))
    (`self.victory_screen`)))

(event `escort_check_alive`
  ;[1 1 1] Escort code
  (`|ExecutionSequence`
    (:`then_0`
      (if (> (`self.enemy_destroyed`) (- (`self.initial_enemy_count`) (`self.num_enemy_get_away`)))
        (set `/Game/Blueprints/GameInstance/game_info_instance.win_or_lose` true (`self.game_inst_ref`))
        (`self.victory_screen`)))
    (:`then_1`
      (if (not (`self.dont_check_allies`))
        (if (> (`self.ally_destroyed`) (- (`self.initial_ally_count`) (`self.num_ally_get_away`)))
          (set `/Game/Blueprints/GameInstance/game_info_instance.win_or_lose` false (`self.game_inst_ref`))
          (`self.victory_screen`))))))

(event `ally_escort_frac`
  ;[1 1 1] Escort code
  (if (not (`self.dont_check_allies`))
    (if (>= (`self.ally_got_away`) (`self.num_ally_get_away`))
      (set `/Game/Blueprints/GameInstance/game_info_instance.win_or_lose` true (`self.game_inst_ref`))
      (`self.victory_screen`))))

(event `escort_remove_enemy`
  (params (InputObject :type "/Game/Blueprints/base_ship Object Reference"))
  ;[1 1 1] Escort code
  (`/Engine/EditorBlueprintResources/StandardMacros.IsValid` InputObject
    (:`Is Valid`
      (if (`self.far_from_origin` InputObject 1000.0)
        (`/Engine/EditorBlueprintResources/StandardMacros.IncrementInt` (`self.enemy_got_away`)
          (:`  `
            (`KismetArrayLibrary.Array_RemoveItem` (`self.all_enemies`) InputObject)
            (`self.K2_DestroyActor` InputObject)))))
    (:`Is Not Valid`
      (`/Engine/EditorBlueprintResources/StandardMacros.IncrementInt` (`self.enemy_destroyed`)
        (:`  `
          (`KismetArrayLibrary.Array_RemoveItem` (`self.all_enemies`) InputObject))))))

(event `escort_remove_ally`
  (params (InputObject :type "/Game/Blueprints/base_ship Object Reference"))
  ;[1 1 1] Escort code
  (`/Engine/EditorBlueprintResources/StandardMacros.IsValid` InputObject
    (:`Is Valid`
      (if (`self.far_from_origin` InputObject 1000.0)
        (`/Engine/EditorBlueprintResources/StandardMacros.IncrementInt` (`self.ally_got_away`)
          (:`  `
            (`KismetArrayLibrary.Array_RemoveItem` (`self.all_allies`) InputObject)
            (`self.K2_DestroyActor` InputObject)))))
    (:`Is Not Valid`
      (`/Engine/EditorBlueprintResources/StandardMacros.IncrementInt` (`self.ally_destroyed`)
        (:`  `
          (`KismetArrayLibrary.Array_RemoveItem` (`self.all_allies`) InputObject))))))

(fn `far_from_origin`
  (params (base_ship :type "/Game/Blueprints/base_ship Object Reference") (`distance [km]` :type "Float (double-precision)"))
  (returns (ReturnValue :type Boolean))
  (return (> (`KismetMathLibrary.VSize` (- (`self.K2_GetActorLocation` base_ship) (0.0 0.0 0.0))) (* `distance [km]` 1000.0 (`/Game/Blueprints/base_ship.scale_factor` base_ship)))))

(fn `init_count`
  (params (TargetArray :type "Array of /Game/Blueprints/base_ship Object Reference (by ref)") (frac :type "Float (double-precision)"))
  (returns (init_count :type Integer) (arrray_length :type Integer))
  (bind _returnvalue (`KismetArrayLibrary.Array_Length` TargetArray))
  (return (`KismetMathLibrary.Clamp` (`KismetMathLibrary.FCeil` (* _returnvalue (`KismetMathLibrary.FClamp` (- 1.0 frac)))) 1 _returnvalue) _returnvalue))

(fn `UserConstructionScript`)