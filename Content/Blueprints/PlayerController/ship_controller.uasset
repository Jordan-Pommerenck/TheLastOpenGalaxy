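; Player controller for a spaceship, mapping gamepad input to flight, primary fire, targeting and energy allocation on the possessed base_ship.
; BeginPlay loads weapon data from a laser table, adds HUD and reticle widgets, and starts looping timers.
; Timed events apply the selected energy allocation and toggle speed-based space particles; engine power engages after a cancellable delay.
; Held fire repeats on a timer, with a DoOnce gate enforcing fire rate.
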(event `Energy Recharge`
  (bind _human_player (`self.human_player`))
  ;[0.25 0.25 0.25] Timer event to control the space particle effect
  (`/Engine/EditorBlueprintResources/StandardMacros.IsValid` _human_player
    (:`Is Valid`
      (switch `Allocation` (`master_ship.energy_allocation` _human_player)
        (:`shields`
          (`master_ship.allocate_to_shields` _human_player))
        (:`weapons`
          (`master_ship.allocate_to_weapons` _human_player))
        (:`systems`
          (`master_ship.allocate_to_systems` _human_player))
        (:`engines`
          (`master_ship.allocate_to_engines` _human_player))))
    (:`Is Not Valid`
      (`KismetSystemLibrary.K2_ClearAndInvalidateTimerHandle` (`self.engine_timer`)))))

(event `Space Particle Effect`
  (bind _space_particles (`self.space_particles`))
  (bind _human_player (`self.human_player`))
  (bind _human_player_2 (`self.human_player`))
  ;[0.25 0.25 0.25] Timer event to control the space particle effect
  (`/Engine/EditorBlueprintResources/StandardMacros.IsValid` _human_player
    (:`Is Valid`
      (if (> (`master_ship.current_speed` _human_player) (* (`master_ship.base_speed` _human_player) 0.5))
        (`/Engine/EditorBlueprintResources/StandardMacros.DoOnce` true :!label _label
          (:`Completed`
            (bind _returnvalue (`|SpawnActorFromClass` "/Game/Particles_Wind_Control_System/Blueprints/BP_Particle_Space.BP_Particle_Space_C" (`KismetMathLibrary.MakeTransform` (673.0 0.0 0.0) (struct :`Pitch` -90.0 :`Yaw` 180.0 :`Roll` 180.0)) "Undefined" "OverrideRootScale" _human_player_2 null))
            (bind _output_get (set `self.space_particles` _returnvalue))
            (`self.K2_AttachToActor` _returnvalue _human_player_2 "space_prt_effect" "KeepRelative" "KeepRelative" "KeepRelative" false)
            (`self.K2_AttachToActor` _output_get _human_player_2 "space_prt_effect" "KeepRelative" "KeepRelative" "KeepRelative" false)))
        (else
          (`/Engine/EditorBlueprintResources/StandardMacros.IsValid` _space_particles
            (:`Is Valid`
              (`self.K2_DetachFromActor` _space_particles "KeepWorld" "KeepWorld" "KeepWorld")
              (`KismetSystemLibrary.Delay` 3.0)
              (`self.K2_DestroyActor` _space_particles)
              (goto _label :!via `Reset`))
            (:`Is Not Valid`
              (goto _label :!via `Reset`))))))))

(event `Key|Q`
  (params (Key :type "Key Structure"))
  ;[1 0 1] DEBUG KEYS
  (:`Pressed`
    (`KismetSystemLibrary.QuitGame` null "Quit")))

(event `self.ReceiveBeginPlay`
  (bind _returnvalue (`self.K2_GetPawn`))
  (bind _human_player (`self.human_player`))
  (`/Engine/EditorBlueprintResources/StandardMacros.IsValid` _returnvalue
    (:`Is Valid`
      (bind _asbase_ship (cast `/Game/Blueprints/base_ship` _returnvalue))
      (bind _output_get (set `self.human_player` _asbase_ship))
      (`self.get_prmy_weap_params` _output_get)
      (`KismetSystemLibrary.K2_SetTimerDelegate` (`|CreateDelegate` :!event `Energy Recharge`) 1.0 true)
      (`KismetSystemLibrary.K2_SetTimerDelegate` (`|CreateDelegate` :!event `Space Particle Effect`) 0.5 true)
      ;[0.25 0.25 0.25] Time for parameters to update for base ship
      (`KismetSystemLibrary.Delay` 0.2)
      (`GameplayStatics.PlaySound2D` (`master_ship.engine_hum` _human_player) 4.0 0.5 0.0 null _human_player)
      (bind _returnvalue_2 (`|CreateWidget` "/Game/Blueprints/UI/HUD/fighter-hud.fighter-hud_C" self))
      (`UserWidget.AddToViewport` _returnvalue_2 0)
      (bind _returnvalue_3 (`|CreateWidget` "/Game/Blueprints/UI/TargetingReticle.TargetingReticle_C" self))
      (`UserWidget.AddToViewport` _returnvalue_3 0))))

(event `Key|Zero`
  (params (Key :type "Key Structure"))
  ;[1 0 1] DEBUG KEYS
  (:`Pressed`
    (set `master_ship.current_systems` 0 (`self.human_player`))))

(event `InputAxisKey|Gamepad_LeftY`
  (params (AxisValue :type "Float (single-precision)"))
  (bind _human_player (`self.human_player`))
  (`/Engine/EditorBlueprintResources/StandardMacros.IsValid` _human_player
    (:`Is Valid`
      (`master_ship.update_pitch` _human_player AxisValue (`GameplayStatics.GetWorldDeltaSeconds`)))))

(event `InputAxisKey|Gamepad_LeftX`
  (params (AxisValue :type "Float (single-precision)"))
  (bind _human_player (`self.human_player`))
  (`/Engine/EditorBlueprintResources/StandardMacros.IsValid` _human_player
    (:`Is Valid`
      (`master_ship.update_yaw` _human_player AxisValue (`GameplayStatics.GetWorldDeltaSeconds`)))))

(event `InputAxisKey|Gamepad_RightX`
  (params (AxisValue :type "Float (single-precision)"))
  (bind _human_player (`self.human_player`))
  (`/Engine/EditorBlueprintResources/StandardMacros.IsValid` _human_player
    (:`Is Valid`
      (`master_ship.update_roll` _human_player AxisValue (`GameplayStatics.GetWorldDeltaSeconds`)))))

(event `InputAxisKey|Gamepad_LeftTriggerAxis`
  (params (AxisValue :type "Float (single-precision)"))
  (bind _human_player (`self.human_player`))
  (`/Engine/EditorBlueprintResources/StandardMacros.IsValid` _human_player
    (:`Is Valid`
      (`master_ship.update_speed` _human_player AxisValue (`GameplayStatics.GetWorldDeltaSeconds`) false)
      (`master_ship.update_speed` _human_player AxisValue (`GameplayStatics.GetWorldDeltaSeconds`) false))))

(event `InputAxisKey|Gamepad_RightTriggerAxis`
  (params (AxisValue :type "Float (single-precision)"))
  (bind _human_player (`self.human_player`))
  (`/Engine/EditorBlueprintResources/StandardMacros.IsValid` _human_player
    (:`Is Valid`
      (`master_ship.update_speed` _human_player AxisValue (`GameplayStatics.GetWorldDeltaSeconds`) true))))

(event `Key|Gamepad_DPad_Up`
  (params (Key :type "Key Structure"))
  (bind _human_player (`self.human_player`))
  (:`Pressed`
    (`/Engine/EditorBlueprintResources/StandardMacros.IsValid` _human_player
      (:`Is Valid`
        (set `master_ship.energy_allocation` "shields" _human_player)
        (`KismetSystemLibrary.K2_ClearAndInvalidateTimerHandle` (`self.engine_timer`) :!label _label_2)
        (`GameplayStatics.PlaySound2D` "/Game/Sci-FiSoundPack/Interface/wav/Digital_Click_13.Digital_Click_13" 1.0 1.0 0.0 null null :!label _label_3)))))

(event `Key|Gamepad_DPad_Down`
  (params (Key :type "Key Structure"))
  (bind _human_player (`self.human_player`))
  (:`Pressed`
    (`/Engine/EditorBlueprintResources/StandardMacros.IsValid` _human_player
      (:`Is Valid`
        (set `master_ship.energy_allocation` "weapons" _human_player)
        (goto _label_2)))))

(event `Key|Gamepad_DPad_Left`
  (params (Key :type "Key Structure"))
  (bind _human_player (`self.human_player`))
  (:`Pressed`
    (`/Engine/EditorBlueprintResources/StandardMacros.IsValid` _human_player
      (:`Is Valid`
        (set `master_ship.energy_allocation` "systems" _human_player)
        (goto _label_2)))))

(event `Key|Gamepad_DPad_Right`
  (params (Key :type "Key Structure"))
  (bind _human_player (`self.human_player`))
  (:`Pressed`
    (`/Engine/EditorBlueprintResources/StandardMacros.IsValid` _human_player
      (:`Is Valid`
        (bind _returnvalue (`KismetSystemLibrary.K2_SetTimerDelegate` (delegate `All Power to Engines`) (`master_ship.hyper_time` _human_player)))
        (set `self.engine_timer` _returnvalue)
        (goto _label_3)))))

(event `All Power to Engines`
  (bind _human_player (`self.human_player`))
  (`/Engine/EditorBlueprintResources/StandardMacros.IsValid` _human_player
    (:`Is Valid`
      (set `master_ship.energy_allocation` "engines" _human_player))))

(event `Fire Weapon`
  (params (`base ship` :type "/Game/Blueprints/base_ship Object Reference"))
  (bind ((`concurrency_16_8AAD35DF4AD910C527DF458D10D22507` _concurrency) (`reload_sound_23_C5FBDE424CACF77958C09A8C754D8926` _reload_sound) (`reload_volume_28_D01073D04792C10F0454AD93B490C354` _reload_volume)) (break `/Game/Data/Structures/laser_params` (`self.prmy_weap_struct`)))
  ;[0.25 0.25 0.25] Fire the primary weapon and handle the case when the button is held down
  (bind _laser_count (`/Game/Blueprints/base_ship.fire_prm_weap` `base ship`))
  (if _laser_count
    (`GameplayStatics.PlaySound2D` _reload_sound _reload_volume 1.0 0.0 _concurrency self)))

(event `Key|Gamepad_FaceButton_Left`
  (params (Key :type "Key Structure"))
  ;[0.25 0.25 0.25] Fire the primary weapon and handle the case when the button is held down
  (:`Pressed`
    (`self.Press Fire`))
  (:`Released`
    (`self.Release Fire`)))

(event `Hold Down Fire`
  (bind _human_player (`self.human_player`))
  ;[0.25 0.25 0.25] Fire the primary weapon and handle the case when the button is held down
  (`/Engine/EditorBlueprintResources/StandardMacros.IsValid` _human_player :!label _label_4
    (:`Is Valid`
      (`self.Fire Weapon` _human_player)
      (bind _returnvalue (`KismetSystemLibrary.K2_SetTimerDelegate` (delegate `Hold Down Fire`) (`master_ship.lsr_fire_rate` _human_player) true))
      (set `self.laser_timer` _returnvalue))))

(event `Press Fire`
  ;[0.25 0.25 0.25] Fire the primary weapon and handle the case when the button is held down
  (`/Engine/EditorBlueprintResources/StandardMacros.DoOnce` false :!label _label_5
    (:`Completed`
      (goto _label_4))))

(event `Release Fire`
  (bind _human_player (`self.human_player`))
  ;[0.25 0.25 0.25] Fire the primary weapon and handle the case when the button is held down
  (`KismetSystemLibrary.K2_ClearAndInvalidateTimerHandle` (`self.laser_timer`))
  (`/Engine/EditorBlueprintResources/StandardMacros.IsValid` _human_player
    (:`Is Valid`
      (`KismetSystemLibrary.Delay` (`master_ship.lsr_fire_rate` _human_player))
      (if (`self.IsInputKeyDown` (stale `Key|Gamepad_FaceButton_Left` Key))
        (`self.Hold Down Fire`)
        (else
          (goto _label_5 :!via `Reset`))))))

(event `Key|Gamepad_FaceButton_Top`
  (params (Key :type "Key Structure"))
  (bind _human_player (`self.human_player`))
  (:`Pressed`
    (`/Engine/EditorBlueprintResources/StandardMacros.IsValid` _human_player
      (:`Is Valid`
        (bind _hit_actor (`/Game/Blueprints/base_ship.find_my_target` _human_player _human_player))
        (set `master_ship.my_target` _hit_actor _human_player)
        (`GameplayStatics.PlaySound2D` "/Game/Binary_Code_2/cues/4_Subtle_Holograms/Interface_Subtle_Hologram_023_Cue.Interface_Subtle_Hologram_023_Cue" 6.0 1.0 0.0 null null)))))

(fn `get_prmy_weap_params`
  (params (base_ship :type "master_ship Object Reference"))
  (bind _returnvalue (`|GetDataTableRow` "/Game/Data/table_laser.table_laser" (`KismetStringLibrary.Conv_StringToName` (`|GetEnumeratorNameAsString` (`master_ship.my_laser_type` base_ship))))
    (:`then`
      (set `self.prmy_weap_struct` _returnvalue)
      (return))
    (:`RowNotFound`
      (`KismetSystemLibrary.PrintString` "Not valid laser type!"))))

(fn `UserConstructionScript`)