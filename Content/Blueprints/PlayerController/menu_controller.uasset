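; Player controller for the menu that orbits and zooms the camera around the Rotate_menu_craft preview actor.
; On BeginPlay it caches that actor and starts a looping timer, apparently to poll for the Craftlibrary widget until found.
; While both references are valid, Tick turns mouse movement into spring arm rotation.
; The mouse wheel changes arm length, scaled by mesh size and clamped to multiples of its bounds radius.
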(event `self.ReceiveEndPlay`
  (params (EndPlayReason :type "EEndPlayReason Enum" :default "Destroyed"))
  (`KismetSystemLibrary.K2_ClearAndInvalidateTimerHandle` (`self.search_timer`)))

(event `self.ReceiveBeginPlay`
  (bind _returnvalue (`KismetSystemLibrary.K2_SetTimerDelegate` (`|CreateDelegate` :!event `look_for_craft_library`) 0.5 true))
  (set `self.search_timer` _returnvalue)
  (bind _outactors (`GameplayStatics.GetAllActorsOfClass` "/Game/Blueprints/menu_render/rotate_menu_craft.rotate_menu_craft_C"))
  (set `self.rotate_menu_actor` (`|GetArrayItem` _outactors)))

(event `look_for_craft_library`
  (bind _foundwidgets (`WidgetBlueprintLibrary.GetAllWidgetsOfClass` "/Game/Blueprints/UI/MainMenu/craft-library.craft-library_C"))
  (if (not (== (`KismetArrayLibrary.Array_Length` _foundwidgets) 0))
    (`KismetSystemLibrary.K2_ClearAndInvalidateTimerHandle` (`self.search_timer`))
    (set `self.craft_library` (`|GetArrayItem` _foundwidgets))))

(event `InputAxisKey|MouseWheelAxis`
  (params (AxisValue :type "Float (single-precision)"))
  (bind _rotate_menu_actor (`self.rotate_menu_actor`))
  (bind _springarm (`/Game/Blueprints/menu_render/rotate_menu_craft.SpringArm` _rotate_menu_actor))
  (bind _staticmesh (`/Game/Blueprints/menu_render/rotate_menu_craft.StaticMesh` _rotate_menu_actor))
  (bind (_origin _boxextent _sphereradius) (`KismetSystemLibrary.GetComponentBounds` _staticmesh))
  (`/Engine/EditorBlueprintResources/StandardMacros.IsValid` (`self.craft_library`)
    (:`Is Valid`
      (`/Engine/EditorBlueprintResources/StandardMacros.IsValid` _rotate_menu_actor
        (:`Is Valid`
          (set `SpringArmComponent.TargetArmLength` (`KismetMathLibrary.FClamp` (+ (`SpringArmComponent.TargetArmLength` _springarm) (* AxisValue 5.0 (.x (`SceneComponent.K2_GetComponentScale` _staticmesh)))) (* _sphereradius 2.25) (* _sphereradius 4.0)) _springarm))))))

(event `self.ReceiveTick`
  (params (DeltaSeconds :type "Float (single-precision)"))
  (bind (_deltax _deltay) (`self.GetInputMouseDelta`))
  (bind _rotate_menu_actor (`self.rotate_menu_actor`))
  (bind _springarm (`/Game/Blueprints/menu_render/rotate_menu_craft.SpringArm` _rotate_menu_actor))
  (`/Engine/EditorBlueprintResources/StandardMacros.IsValid` (`self.craft_library`)
    (:`Is Valid`
      (`/Engine/EditorBlueprintResources/StandardMacros.IsValid` _rotate_menu_actor
        (:`Is Valid`
          (`SceneComponent.K2_SetWorldRotation` _springarm (`KismetMathLibrary.ComposeRotators` (`SceneComponent.K2_GetComponentRotation` _springarm) (`KismetMathLibrary.MakeRotator` 0.0 (* _deltay -1.0) _deltax)) false false))))))

(fn `UserConstructionScript`)