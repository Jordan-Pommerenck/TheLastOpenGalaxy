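; Base ship class that loads stats, weapon slots and scale from a data table by row name.
; Lasers drain shields, then spill into systems (blue types) or hull, while missiles bypass shields.
; Ship collisions push back and cost hull by relative scale; depleted hull triggers an explosion.
; Firing aims from an Arrow, leading in-range targets using table-cached weapon speeds, and per-slot counters cycle through locations.
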(event `self.ReceiveBeginPlay`)

(event `explosion_death`
  (`GameplayStatics.PlaySoundAtLocation` "/Game/PremiumBeat/Explosions/0050_explosion_blast_5_PremiumBeat.0050_explosion_blast_5_PremiumBeat" (`self.K2_GetActorLocation` self) (struct) 5.0 (`KismetMathLibrary.FClamp` (/ 100.0 (`self.base_scale`)) 0.1) 0.0 "/Game/Audio/attenuation_big_explosion.attenuation_big_explosion" null self)
  (`ActorComponent.K2_DestroyComponent` (`self.StaticMesh`))
  (`KismetSystemLibrary.Delay` 1.0)
  (`self.K2_DestroyActor`))

(event `self.ReceiveAnyDamage`
  (params (Damage :type "Float (single-precision)") (DamageType :type "DamageType Object Reference") (InstigatedBy :type "Controller Object Reference") (DamageCauser :type "Actor Object Reference"))
  (bind _hit_weapon_type (`self.hit_weapon_type`))
  (bind _returnvalue (- (`self.current_shields`) (`KismetMathLibrary.FTrunc` Damage)))
  (bind _returnvalue_2 (`KismetMathLibrary.Abs_Int` _returnvalue))
  ;[0.25 0.25 0.25] Shield and Hull damage when hit by a Weapon
  (`/Engine/EditorBlueprintResources/StandardMacros.IsValid` DamageCauser
    (:`Is Valid`
      (bind _aslaser (cast `/Game/Blueprints/Weapons/laser` DamageCauser))
      (set `self.hit_weapon_type` (`/Game/Blueprints/Weapons/laser.laser_type` _aslaser))
      (if (not (`/Game/Blueprints/Weapons/laser.missile` _aslaser))
        (if (>= _returnvalue 0)
          (set `self.current_shields` _returnvalue)
          (elif (or (`|EnumEquality` _hit_weapon_type "lgtblue") (`|EnumEquality` _hit_weapon_type "medblue") (`|EnumEquality` _hit_weapon_type "hvyblue") (`|EnumEquality` _hit_weapon_type "megablue"))
            (set `self.current_shields` 0)
            (`self.calculate_systems_damage` _returnvalue_2)
            (else
              (set `self.current_shields` 0)
              (`self.calculate_hull_damage` _returnvalue_2)
              (if (<= (`self.current_hull`) 0) :!label _label
                (`self.explosion_death`)))))
        (else
          (`self.calculate_hull_damage` (`KismetMathLibrary.FTrunc` Damage) :!label _label_2)
          (if (<= (`self.current_hull`) 0)
            (`self.explosion_death`)))))
    (:`Is Not Valid`
      (goto _label_2))))

(event `self.ReceiveHit`
  (params (MyComp :type "PrimitiveComponent Object Reference") (Other :type "Actor Object Reference") (OtherComp :type "PrimitiveComponent Object Reference") (bSelfMoved :type Boolean) (HitLocation :type "Vector Structure") (HitNormal :type "Vector Structure") (NormalImpulse :type "Vector Structure") (Hit :type "HitResult Structure (by ref)"))
  (set `self.taking_damage` true)
  (`/Engine/EditorBlueprintResources/StandardMacros.IsValid` Other
    (:`Is Valid`
      (cast `/Game/Blueprints/Weapons/laser` Other
        (:`CastFailed`
          (bind _asbase_ship (cast `/Game/Blueprints/base_ship` Other))
          (`self.K2_SetActorLocationAndRotation` (+ (* HitNormal (`.SphereRadius` (`KismetSystemLibrary.GetComponentBounds` (`self.StaticMesh`)))) (`self.K2_GetActorLocation` self)) (`KismetMathLibrary.Conv_VectorToRotator` (`KismetMathLibrary.NegateVector` HitNormal)) false true)
          (set `self.current_hull` (- (`self.current_hull`) (`KismetMathLibrary.FTrunc` (* (/ (`master_ship.base_scale` _asbase_ship) (+ (`self.base_scale`) 1.0)) (* (`self.base_hull`) 0.1)))))
          (`|ExecutionSequence`
            (:`then_0`
              (bind _asship_controller (cast `/Game/Blueprints/PlayerController/ship_controller` (`self.GetController` self)))
              (`/Game/Blueprints/PlayerController/ship_controller.sound_on_collision` _asship_controller))
            (:`then_1`
              (goto _label))))))))

(fn `find_my_target`
  (params (base_ship :type "Actor Object Reference"))
  (returns (hit_actor :type "/Game/Blueprints/base_ship Object Reference"))
  (bind _returnvalue (`self.K2_GetActorLocation` base_ship))
  (bind _scale_factor (`self.scale_factor`))
  (bind _outhit (`KismetSystemLibrary.SphereTraceSingleForObjects` _returnvalue (+ _returnvalue (* (`self.GetActorForwardVector` base_ship) (* 50.0 _scale_factor 1000.0))) (* _scale_factor 25.0) (`|MakeArray` "ObjectTypeQuery1" :!type "EObjectTypeQuery Enum") false (`|MakeArray` base_ship)))
  (bind (_bblockinghit _binitialoverlap _time _distance _location _impactpoint _normal _impactnormal _physmat _hitactor) (`GameplayStatics.BreakHitResult` _outhit))
  (`/Engine/EditorBlueprintResources/StandardMacros.IsValid` _hitactor
    (:`Is Valid`
      (bind _asbase_ship (cast `/Game/Blueprints/base_ship` _hitactor))
      (return _asbase_ship))))

(fn `fire_weapon`
  (params (weapon_locations :type "Array of Vector Structure") (count :type Integer))
  (bind _arrow (`self.Arrow`))
  (`self.focus_weapon`)
  (bind _returnvalue (`|SpawnActorFromClass` "/Game/Blueprints/Weapons/laser.laser_C" (`KismetMathLibrary.MakeTransform` (.location (`SceneComponent.K2_GetComponentToWorld` _arrow)) (`self.arrow_rotation`) (.scale (`SceneComponent.K2_GetComponentToWorld` _arrow))) "Undefined" "OverrideRootScale" null self))
  (set `master_laser.base_speed` (+ (`master_laser.base_speed` _returnvalue) (`self.current_speed`)) _returnvalue)
  (`SceneComponent.K2_SetRelativeLocation` _arrow (`|GetArrayItem` weapon_locations count) false false)
  (return))

(fn `focus_weapon`
  (bind _my_target (`self.my_target`))
  (bind _arrow (`self.Arrow`))
  (bind _my_target_2 (`self.my_target`))
  (bind _returnvalue (`SceneComponent.K2_GetComponentLocation` _arrow))
  (`/Engine/EditorBlueprintResources/StandardMacros.IsValid` _my_target
    (:`Is Valid`
      (bind _in_range (`self.in_range` _my_target 0.99))
      (if _in_range
        (bind _asbase_ship (cast `/Game/Blueprints/base_ship` _my_target_2)
          (:`then`
            (set `self.arrow_rotation` (`KismetMathLibrary.FindLookAtRotation` _returnvalue (+ (`self.K2_GetActorLocation` _asbase_ship) (* (`self.GetActorForwardVector` _asbase_ship) (* (`master_ship.current_speed` _asbase_ship) (/ (`KismetMathLibrary.VSize` (- _returnvalue (`self.K2_GetActorLocation` _my_target_2))) (`|GetArrayItem` (`self.weapon_velocities`) (`KismetMathLibrary.Conv_ByteToInt` (`KismetSystemLibrary.MakeLiteralByte` (`self.which_weapon`)))))))))))
          (:`CastFailed`
            (set `self.arrow_rotation` (`SceneComponent.K2_GetComponentRotation` _arrow) :!label _label)))
        (else
          (goto _label))))
    (:`Is Not Valid`
      (goto _label)))
  (return))

(fn `in_range`
  (params (my_target :type "Actor Object Reference") (target_factor :type "Float (double-precision)"))
  (returns (in_range :type Boolean))
  (return (and (>= (`KismetMathLibrary.Dot_VectorVector` (`KismetMathLibrary.Normal` (- (`self.K2_GetActorLocation` my_target) (`self.K2_GetActorLocation` self))) (`self.GetActorForwardVector` self)) target_factor) (< (`self.GetDistanceTo` self my_target) (* (`self.scale_factor`) 1000.0 1.0)))))

(fn `initialize_base_params`
  (params (which_ship :type Name))
  (bind _scale_factor (`self.scale_factor`))
  (bind _returnvalue (`|GetDataTableRow` "/Game/Data/table_bsp.table_bsp" which_ship)
    (:`then`
      (bind (_my_name _base_yaw _base_pitch _base_roll _base_speed _base_accel _base_hull _base_shields _base_systems _base_lasers _base_warheads _shd_rchrg _lsr_rchrg _sys_rchrg _hyper_rot _hyper_speed _hyper_accel _hyper_time _base_scale _collision_diameter _prmy_fire_rate _scdy_fire_rate _trty_fire_rate _qtry_fire_rate _qnry_fire_rate _snry_fire_rate _spty_fire_rate _octy_fire_rate _nnry_fire_rate _dnry_fire_rate _prmy_locations _scdy_locations _trty_locations _qtry_locations _qnry_locations _snry_locations _spty_locations _octy_locations _nnry_locations _dnry_locations _engine_hum _my_team _my_class _prmy_weap_typelasers _scdy_weap_typelasers _trty_weap_typewarheads _qtry_weap_typewarheads _qnry_weap_typewarheads _snry_weap_typewarheads _spty_weap_typelasers _octy_weap_typelasers _nnry_weap_typelasers _dnry_weap_typelasers) (break `/Game/Data/Structures/base_ship_params` _returnvalue))
      (set `self.base_yaw` _base_yaw)
      (set `self.base_pitch` _base_pitch)
      (set `self.base_roll` _base_roll)
      (set `self.base_speed` (* _scale_factor _base_speed))
      (set `self.base_acceleration` (* _scale_factor _base_accel))
      (set `self.prmy_fire_rate` _prmy_fire_rate)
      (set `self.scdy_fire_rate` _scdy_fire_rate)
      (set `self.trty_fire_rate` _trty_fire_rate)
      (bind _output_get (set `self.base_hull` _base_hull))
      (bind _output_get_2 (set `self.base_shields` _base_shields))
      (bind _output_get_3 (set `self.base_systems` _base_systems))
      (bind _output_get_4 (set `self.base_lasers` _base_lasers))
      (set `self.shd_rchrg` _shd_rchrg)
      (set `self.lsr_rchrg` _lsr_rchrg)
      (set `self.sys_rchrg` _sys_rchrg)
      (set `self.hyper_rot_factor` _hyper_rot)
      (set `self.hyper_speed` (* _scale_factor _hyper_speed))
      (set `self.hyper_accel` (* _scale_factor _hyper_accel))
      (set `self.hyper_time` _hyper_time)
      (set `self.prmy_locations` _prmy_locations)
      (set `self.scdy_locations` _scdy_locations)
      (set `self.trty_locations` _trty_locations)
      (set `self.collision_diameter` _collision_diameter)
      (set `self.current_hull` _output_get)
      (set `self.current_shields` _output_get_2)
      (set `self.current_systems` _output_get_3)
      (set `self.current_lasers` _output_get_4)
      (bind _output_get_5 (set `self.base_scale` _base_scale))
      (set `self.engine_hum` _engine_hum)
      (set `self.my_name` _my_name)
      (set `self.my_team` _my_team)
      (set `self.my_class` _my_class)
      (set `self.prmy_weap_type` _prmy_weap_typelasers)
      (set `self.scdy_weap_type` _scdy_weap_typelasers)
      (set `self.trty_weap_type` _trty_weap_typewarheads)
      (bind _output_get_6 (set `self.base_warheads` _base_warheads))
      (set `self.current_warheads` _output_get_6)
      (set `self.qtry_locations` _qtry_locations)
      (set `self.qnry_locations` _qnry_locations)
      (set `self.snry_locations` _snry_locations)
      (set `self.spty_locations` _spty_locations)
      (set `self.octy_locations` _octy_locations)
      (set `self.nnry_locations` _nnry_locations)
      (set `self.dnry_locations` _dnry_locations)
      (set `self.qtry_weap_type` _qtry_weap_typewarheads)
      (set `self.qnry_weap_type` _qnry_weap_typewarheads)
      (set `self.snry_weap_type` _snry_weap_typewarheads)
      (set `self.spty_weap_type` _spty_weap_typelasers)
      (set `self.octy_weap_type` _octy_weap_typelasers)
      (set `self.nnry_weap_type` _nnry_weap_typelasers)
      (set `self.dnry_weap_type` _dnry_weap_typelasers)
      (set `self.qtry_fire_rate` _qtry_fire_rate)
      (set `self.qnry_fire_rate` _qnry_fire_rate)
      (set `self.snry_fire_rate` _snry_fire_rate)
      (set `self.spty_fire_rate` _spty_fire_rate)
      (set `self.octy_fire_rate` _octy_fire_rate)
      (set `self.nnry_fire_rate` _nnry_fire_rate)
      (set `self.dnry_fire_rate` _dnry_fire_rate)
      (`self.set_scale` (`self.StaticMesh`) _output_get_5)
      (`self.initialize_wpn_speeds`))))

(fn `initialize_wpn_speeds`
  (bind _weapon_velocities (`self.weapon_velocities`))
  (bind _weapon_velocities_2 (`self.weapon_velocities`))
  (bind _weapon_velocities_3 (`self.weapon_velocities`))
  (bind _weapon_velocities_4 (`self.weapon_velocities`))
  (bind _weapon_velocities_5 (`self.weapon_velocities`))
  (bind _weapon_velocities_6 (`self.weapon_velocities`))
  (bind _weapon_velocities_7 (`self.weapon_velocities`))
  (bind _weapon_velocities_8 (`self.weapon_velocities`))
  (bind _weapon_velocities_9 (`self.weapon_velocities`))
  (bind _weapon_velocities_10 (`self.weapon_velocities`))
  (`|ExecutionSequence`
    (:`then_0`
      (bind _returnvalue (`|GetDataTableRow` "/Game/Data/table_laser.table_laser" (`KismetStringLibrary.Conv_StringToName` (`|GetEnumeratorNameAsString` (`self.prmy_weap_type`))))
        (:`then`
          (`KismetArrayLibrary.Array_Add` _weapon_velocities_2 (`.base_speed_2_87C7E2804B59922F68F0EFAA4E673EA8` (break `/Game/Data/Structures/laser_params` _returnvalue))))
        (:`RowNotFound`
          (`KismetArrayLibrary.Array_Add` _weapon_velocities_2))))
    (:`then_1`
      (bind _returnvalue_2 (`|GetDataTableRow` "/Game/Data/table_laser.table_laser" (`KismetStringLibrary.Conv_StringToName` (`|GetEnumeratorNameAsString` (`self.scdy_weap_type`))))
        (:`then`
          (`KismetArrayLibrary.Array_Add` _weapon_velocities_3 (`.base_speed_2_87C7E2804B59922F68F0EFAA4E673EA8` (break `/Game/Data/Structures/laser_params` _returnvalue_2))))
        (:`RowNotFound`
          (`KismetArrayLibrary.Array_Add` _weapon_velocities_3))))
    (:`then_2`
      (bind _returnvalue_3 (`|GetDataTableRow` "/Game/Data/table_laser.table_laser" (`KismetStringLibrary.Conv_StringToName` (`|GetEnumeratorNameAsString` (`self.trty_weap_type`))))
        (:`then`
          (`KismetArrayLibrary.Array_Add` _weapon_velocities_4 (`.base_speed_2_87C7E2804B59922F68F0EFAA4E673EA8` (break `/Game/Data/Structures/laser_params` _returnvalue_3))))
        (:`RowNotFound`
          (`KismetArrayLibrary.Array_Add` _weapon_velocities_4))))
    (:`then_3`
      (bind _returnvalue_4 (`|GetDataTableRow` "/Game/Data/table_laser.table_laser" (`KismetStringLibrary.Conv_StringToName` (`|GetEnumeratorNameAsString` (`self.qtry_weap_type`))))
        (:`then`
          (`KismetArrayLibrary.Array_Add` _weapon_velocities_5 (`.base_speed_2_87C7E2804B59922F68F0EFAA4E673EA8` (break `/Game/Data/Structures/laser_params` _returnvalue_4))))
        (:`RowNotFound`
          (`KismetArrayLibrary.Array_Add` _weapon_velocities_5))))
    (:`then_4`
      (bind _returnvalue_5 (`|GetDataTableRow` "/Game/Data/table_laser.table_laser" (`KismetStringLibrary.Conv_StringToName` (`|GetEnumeratorNameAsString` (`self.qnry_weap_type`))))
        (:`then`
          (`KismetArrayLibrary.Array_Add` _weapon_velocities_6 (`.base_speed_2_87C7E2804B59922F68F0EFAA4E673EA8` (break `/Game/Data/Structures/laser_params` _returnvalue_5))))
        (:`RowNotFound`
          (`KismetArrayLibrary.Array_Add` _weapon_velocities_6))))
    (:`then_5`
      (bind _returnvalue_6 (`|GetDataTableRow` "/Game/Data/table_laser.table_laser" (`KismetStringLibrary.Conv_StringToName` (`|GetEnumeratorNameAsString` (`self.snry_weap_type`))))
        (:`then`
          (`KismetArrayLibrary.Array_Add` _weapon_velocities_7 (`.base_speed_2_87C7E2804B59922F68F0EFAA4E673EA8` (break `/Game/Data/Structures/laser_params` _returnvalue_6))))
        (:`RowNotFound`
          (`KismetArrayLibrary.Array_Add` _weapon_velocities_7))))
    (:`then_6`
      (bind _returnvalue_7 (`|GetDataTableRow` "/Game/Data/table_laser.table_laser" (`KismetStringLibrary.Conv_StringToName` (`|GetEnumeratorNameAsString` (`self.spty_weap_type`))))
        (:`then`
          (`KismetArrayLibrary.Array_Add` _weapon_velocities_8 (`.base_speed_2_87C7E2804B59922F68F0EFAA4E673EA8` (break `/Game/Data/Structures/laser_params` _returnvalue_7))))
        (:`RowNotFound`
          (`KismetArrayLibrary.Array_Add` _weapon_velocities_8))))
    (:`then_7`
      (bind _returnvalue_8 (`|GetDataTableRow` "/Game/Data/table_laser.table_laser" (`KismetStringLibrary.Conv_StringToName` (`|GetEnumeratorNameAsString` (`self.octy_weap_type`))))
        (:`then`
          (`KismetArrayLibrary.Array_Add` _weapon_velocities_9 (`.base_speed_2_87C7E2804B59922F68F0EFAA4E673EA8` (break `/Game/Data/Structures/laser_params` _returnvalue_8))))
        (:`RowNotFound`
          (`KismetArrayLibrary.Array_Add` _weapon_velocities_9))))
    (:`then_8`
      (bind _returnvalue_9 (`|GetDataTableRow` "/Game/Data/table_laser.table_laser" (`KismetStringLibrary.Conv_StringToName` (`|GetEnumeratorNameAsString` (`self.nnry_weap_type`))))
        (:`then`
          (`KismetArrayLibrary.Array_Add` _weapon_velocities_10 (`.base_speed_2_87C7E2804B59922F68F0EFAA4E673EA8` (break `/Game/Data/Structures/laser_params` _returnvalue_9))))
        (:`RowNotFound`
          (`KismetArrayLibrary.Array_Add` _weapon_velocities_10))))
    (:`then_9`
      (bind _returnvalue_10 (`|GetDataTableRow` "/Game/Data/table_laser.table_laser" (`KismetStringLibrary.Conv_StringToName` (`|GetEnumeratorNameAsString` (`self.dnry_weap_type`))))
        (:`then`
          (`KismetArrayLibrary.Array_Add` _weapon_velocities (`.base_speed_2_87C7E2804B59922F68F0EFAA4E673EA8` (break `/Game/Data/Structures/laser_params` _returnvalue_10))))
        (:`RowNotFound`
          (`KismetArrayLibrary.Array_Add` _weapon_velocities))))
    (:`then_10`
      (return))))

(fn `set_dnry_count`
  (params (TargetArray :type "Array of Vector Structure (by ref)"))
  (returns (weapon_count :type Boolean))
  (bind _dnry_count (`self.dnry_count`))
  (bind _returnvalue (>= _dnry_count (- (`KismetArrayLibrary.Array_Length` TargetArray) 1)))
  (if _returnvalue
    (set `self.dnry_count` 0)
    (else
      (set `self.dnry_count` (+ _dnry_count 1))))
  (return _returnvalue))

(fn `set_nnry_count`
  (params (TargetArray :type "Array of Vector Structure (by ref)"))
  (returns (weapon_count :type Boolean))
  (bind _nnry_count (`self.nnry_count`))
  (bind _returnvalue (>= _nnry_count (- (`KismetArrayLibrary.Array_Length` TargetArray) 1)))
  (if _returnvalue
    (set `self.nnry_count` 0)
    (else
      (set `self.nnry_count` (+ _nnry_count 1))))
  (return _returnvalue))

(fn `set_octy_count`
  (params (TargetArray :type "Array of Vector Structure (by ref)"))
  (returns (weapon_count :type Boolean))
  (bind _octy_count (`self.octy_count`))
  (bind _returnvalue (>= _octy_count (- (`KismetArrayLibrary.Array_Length` TargetArray) 1)))
  (if _returnvalue
    (set `self.octy_count` 0)
    (else
      (set `self.octy_count` (+ _octy_count 1))))
  (return _returnvalue))

(fn `set_prmy_count`
  (params (TargetArray :type "Array of Vector Structure (by ref)"))
  (returns (weapon_count :type Boolean))
  (bind _prmy_count (`self.prmy_count`))
  (bind _returnvalue (>= _prmy_count (- (`KismetArrayLibrary.Array_Length` TargetArray) 1)))
  (if _returnvalue
    (set `self.prmy_count` 0)
    (else
      (set `self.prmy_count` (+ _prmy_count 1))))
  (return _returnvalue))

(fn `set_qnry_count`
  (params (TargetArray :type "Array of Vector Structure (by ref)"))
  (returns (weapon_count :type Boolean))
  (bind _qnry_count (`self.qnry_count`))
  (bind _returnvalue (>= _qnry_count (- (`KismetArrayLibrary.Array_Length` TargetArray) 1)))
  (if _returnvalue
    (set `self.qnry_count` 0)
    (else
      (set `self.qnry_count` (+ _qnry_count 1))))
  (return _returnvalue))

(fn `set_qtry_count`
  (params (TargetArray :type "Array of Vector Structure (by ref)"))
  (returns (weapon_count :type Boolean))
  (bind _qtry_count (`self.qtry_count`))
  (bind _returnvalue (>= _qtry_count (- (`KismetArrayLibrary.Array_Length` TargetArray) 1)))
  (if _returnvalue
    (set `self.qtry_count` 0)
    (else
      (set `self.qtry_count` (+ _qtry_count 1))))
  (return _returnvalue))

(fn `set_scale`
  (params (base_ship :type "StaticMeshComponent Object Reference") (`scale in meters` :type "Float (double-precision)"))
  (bind (_min _max) (`StaticMeshComponent.GetLocalBounds` base_ship))
  (bind _returnvalue (/ (* `scale in meters` (`self.scale_factor`)) (.x (- _max _min))))
  (set `self.adj_scale` (/ 1.0 _returnvalue))
  (`self.SetActorScale3D` (`KismetMathLibrary.Conv_DoubleToVector` _returnvalue))
  (return))

(fn `set_scdy_count`
  (params (TargetArray :type "Array of Vector Structure (by ref)"))
  (returns (weapon_count :type Boolean))
  (bind _scdy_count (`self.scdy_count`))
  (bind _returnvalue (>= _scdy_count (- (`KismetArrayLibrary.Array_Length` TargetArray) 1)))
  (if _returnvalue
    (set `self.scdy_count` 0)
    (else
      (set `self.scdy_count` (+ _scdy_count 1))))
  (return _returnvalue))

(fn `set_snry_count`
  (params (TargetArray :type "Array of Vector Structure (by ref)"))
  (returns (weapon_count :type Boolean))
  (bind _snry_count (`self.snry_count`))
  (bind _returnvalue (>= _snry_count (- (`KismetArrayLibrary.Array_Length` TargetArray) 1)))
  (if _returnvalue
    (set `self.snry_count` 0)
    (else
      (set `self.snry_count` (+ _snry_count 1))))
  (return _returnvalue))

(fn `set_spty_count`
  (params (TargetArray :type "Array of Vector Structure (by ref)"))
  (returns (weapon_count :type Boolean))
  (bind _spty_count (`self.spty_count`))
  (bind _returnvalue (>= _spty_count (- (`KismetArrayLibrary.Array_Length` TargetArray) 1)))
  (if _returnvalue
    (set `self.spty_count` 0)
    (else
      (set `self.spty_count` (+ _spty_count 1))))
  (return _returnvalue))

(fn `set_trty_count`
  (params (TargetArray :type "Array of Vector Structure (by ref)"))
  (returns (weapon_count :type Boolean))
  (bind _trty_count (`self.trty_count`))
  (bind _returnvalue (>= _trty_count (- (`KismetArrayLibrary.Array_Length` TargetArray) 1)))
  (if _returnvalue
    (set `self.trty_count` 0)
    (else
      (set `self.trty_count` (+ _trty_count 1))))
  (return _returnvalue))

(fn `UserConstructionScript`)