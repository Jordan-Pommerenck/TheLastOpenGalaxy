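; Projectile actor for ship weapons, serving as primary, secondary or tertiary fire from the instigating base_ship.
; BeginPlay loads the weapon's data table row for mesh, sound, damage and speed, adding ship speed to velocity.
; A forward sphere trace finds the likely target to derive lifespan; tertiary shots add a missile tail and home on the ship's target.
; Hits apply damage, then show a shield or explosion effect by remaining shields before destruction.
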(event `SET LIFESPAN`
  (bind _base_speed (`self.base_speed`))
  (`/Engine/EditorBlueprintResources/StandardMacros.IsValid` (`self.hit_actor`)
    (:`Is Valid`
      (set `self.base_lifespan` (`KismetMathLibrary.FClamp` (/ (`self.target_distance`) (* _base_speed (+ (`KismetMathLibrary.RandomFloat`) 0.5))) (* _base_speed 0.5) _base_speed)))
    (:`Is Not Valid`
      _))
  (`KismetSystemLibrary.K2_SetTimerDelegate` (`|CreateDelegate` :!event `Spawn Explosion`) (`self.base_lifespan`)))

(event `SET SCALE`
  (bind _laser (`self.Laser`))
  (`SceneComponent.SetWorldScale3D` _laser (* (`SceneComponent.K2_GetComponentScale` _laser) (`self.base_scale`))))

(event `SET VELOCITY`
  (bind _base_ship (`self.base_ship`))
  (bind _base_speed (`self.base_speed`))
  (`/Engine/EditorBlueprintResources/StandardMacros.IsValid` _base_ship
    (:`Is Valid`
      (`ProjectileMovementComponent.SetVelocityInLocalSpace` (`self.ProjectileMovement`) (`KismetMathLibrary.MakeVector` (`KismetMathLibrary.FClamp` (+ (`master_ship.current_speed` _base_ship) _base_speed) _base_speed (* _base_speed 5.0)))))))

(event `self.ReceiveBeginPlay`
  (bind _instigator (`self.Instigator`))
  (set `self.controller` (`self.GetInstigatorController` _instigator))
  (bind _asbase_ship (cast `/Game/Blueprints/base_ship` _instigator))
  (bind _output_get (set `self.base_ship` _asbase_ship))
  (`self.DETERMINE HIT TARGET`)
  (switch `Weapon_Select` (`master_ship.which_weapon` _output_get)
    (:`primary`
      (bind _returnvalue (`|GetDataTableRow` "/Game/Data/table_laser.table_laser" (`KismetStringLibrary.Conv_StringToName` (`|GetEnumeratorNameAsString` (`master_ship.prmy_weap_type` _asbase_ship))))
        (:`then`
          (set `self.laser_params` _returnvalue))))
    (:`secondary`
      (bind _returnvalue_2 (`|GetDataTableRow` "/Game/Data/table_laser.table_laser" (`KismetStringLibrary.Conv_StringToName` (`|GetEnumeratorNameAsString` (`master_ship.scdy_weap_type` _asbase_ship))))
        (:`then`
          (set `self.laser_params` _returnvalue_2))))
    (:`tertiary`
      (bind _returnvalue_3 (`|GetDataTableRow` "/Game/Data/table_laser.table_laser" (`KismetStringLibrary.Conv_StringToName` (`|GetEnumeratorNameAsString` (`master_ship.trty_weap_type` _asbase_ship))))
        (:`then`
          (bind _output_get_2 (set `self.laser_params` _returnvalue_3))
          (bind ((`missile_tail_47_D227B8C440A576DBE71484AC2FA899D3` _missile_tail) (`missile_tail_scale_51_C86AD84740A1856AF65AC2AD8E1964DE` _missile_tail_scale)) (break `/Game/Data/Structures/laser_params` _output_get_2))
          (`self.Spawn Warhead Tail` _missile_tail _missile_tail_scale)))))
  (bind (_attenuation _concurrency) (`self.init_laser_params` (`self.laser_params`)))
  (`GameplayStatics.PlaySoundAtLocation` (`self.laser_sound`) (`SceneComponent.K2_GetComponentLocation` (`self.Laser`)) (struct) (`self.laser_volume`) 1.0 0.0 _attenuation _concurrency null)
  (`self.SET LIFESPAN`)
  (`self.SET VELOCITY`)
  (`self.SET SCALE`))

(event `DETERMINE HIT TARGET`
  (bind _laser (`self.Laser`))
  (bind _returnvalue (`SceneComponent.K2_GetComponentLocation` _laser))
  ;[0.25 0.25 0.25] Determine what target will be hit (Return Hit Actor)
  (bind _outhit (`KismetSystemLibrary.SphereTraceSingleForObjects` _returnvalue (+ _returnvalue (* (`SceneComponent.GetForwardVector` _laser) 100000.0)) 50.0 (`|MakeArray` "ObjectTypeQuery1" :!type "EObjectTypeQuery Enum") false (`|MakeArray` (`self.Instigator`) :!type "Actor Object Reference")))
  (bind (_bblockinghit _binitialoverlap _time _distance _location _impactpoint _normal _impactnormal _physmat _hitactor) (`GameplayStatics.BreakHitResult` _outhit))
  (`/Engine/EditorBlueprintResources/StandardMacros.IsValid` _hitactor
    (:`Is Valid`
      (bind _output_get (set `self.hit_actor` _hitactor))
      (set `self.target_distance` (`self.GetDistanceTo` _output_get (`self.base_ship`))))))

(event `Spawn Warhead Tail`
  (params (missile_tail :type "ParticleSystem Object Reference") (missile_scale :type "Float (double-precision)"))
  (bind _projectilemovement (`self.ProjectileMovement`))
  (bind _my_target (`master_ship.my_target` (`self.base_ship`)))
  (`GameplayStatics.SpawnEmitterAttached` missile_tail (`self.Laser`) "None" (-120.0 0.0 0.0) (struct) (`KismetMathLibrary.Conv_DoubleToVector` missile_scale))
  (`/Engine/EditorBlueprintResources/StandardMacros.IsValid` _my_target
    (:`Is Valid`
      (set `ProjectileMovementComponent.bIsHomingProjectile` true _projectilemovement)
      (set `ProjectileMovementComponent.HomingTargetComponent` (`Actor.RootComponent` _my_target) _projectilemovement))))

(event `self.ReceiveHit`
  (params (MyComp :type "PrimitiveComponent Object Reference") (Other :type "Actor Object Reference") (OtherComp :type "PrimitiveComponent Object Reference") (bSelfMoved :type Boolean) (HitLocation :type "Vector Structure") (HitNormal :type "Vector Structure") (NormalImpulse :type "Vector Structure") (Hit :type "HitResult Structure (by ref)"))
  (`/Engine/EditorBlueprintResources/StandardMacros.IsValid` Other
    (:`Is Valid`
      (`GameplayStatics.ApplyDamage` Other (`self.base_damage`) (`self.controller`) self)
      (bind _asbase_ship (cast `/Game/Blueprints/base_ship` Other)
        (:`then`
          (if (> (`master_ship.current_shields` _asbase_ship) 0)
            (`self.Spawn Shield`)
            (else
              (`self.Spawn Explosion` :!label _label))))
        (:`CastFailed`
          (goto _label))))
    (:`Is Not Valid`
      (goto _label))))

(event `Spawn Explosion`
  (bind _location (.location (`self.GetTransform`)))
  (bind _rotation (.rotation (`self.GetTransform`)))
  ;[0.25 0.25 0.25] Explosion and Shield Handler
  (set `self.no_hit` false)
  (`GameplayStatics.PlaySoundAtLocation` "/Game/PremiumBeat/Explosions/0017_explo_grenade_06_PremiumBeat.0017_explo_grenade_06_PremiumBeat" _location _rotation 1.0 1.0 0.0 "/Game/Audio/Attenuation_Explosion.Attenuation_Explosion" "/Game/Audio/Default-Concurrency.Default-Concurrency" null)
  (bind _returnvalue (`GameplayStatics.SpawnEmitterAtLocation` "/Game/Explosions/Particles/P_Explosive7.P_Explosive7" _location _rotation (`KismetMathLibrary.Conv_DoubleToVector` 0.4) false))
  (`ActorComponent.K2_DestroyComponent` (`self.Laser`))
  ;;[0 0 0] Lifetime of Explosion
  (`KismetSystemLibrary.Delay` 1.5)
  (`ActorComponent.K2_DestroyComponent` _returnvalue)
  (`self.K2_DestroyActor`))

(event `Spawn Shield`
  (bind _location (.location (`self.GetTransform`)))
  (bind _rotation (.rotation (`self.GetTransform`)))
  ;[0.25 0.25 0.25] Explosion and Shield Handler
  (`GameplayStatics.PlaySoundAtLocation` "/Game/Sci-FiSoundPack/Electric/cue/Shield_Device_2_Stop_Cue.Shield_Device_2_Stop_Cue" _location _rotation 5.0 1.0 0.0 "/Game/Audio/Attenuation_Explosion.Attenuation_Explosion" "/Game/Audio/Default-Concurrency.Default-Concurrency" null)
  (bind _returnvalue (`GameplayStatics.SpawnEmitterAtLocation` "/Game/Explosions/Particles/ShieldHit.ShieldHit" _location _rotation (`KismetMathLibrary.Conv_DoubleToVector` 0.2) false))
  (`ActorComponent.K2_DestroyComponent` (`self.Laser`))
  ;;[0 0 0] Lifetime of Explosion
  (`KismetSystemLibrary.Delay` 0.5)
  (`ActorComponent.K2_DestroyComponent` _returnvalue)
  (`self.K2_DestroyActor`))

(fn `init_laser_params`
  (params (laser_params :type "/Game/Data/Structures/laser_params Structure (by ref)"))
  (returns (attenuation :type "SoundAttenuation Object Reference") (concurrency :type "SoundConcurrency Object Reference"))
  (locals (NewLocalVar_0 :type "MaterialInterface Object Reference" :default "MaterialInstanceConstant'/Game/Materials/MI_laser_blue.MI_laser_blue'"))
  (bind (_base_speed _base_damage _base_lifespan _scale _weapon_sound _weapon_volume _attenuation _concurrency _reload_sound _reload_volume _weapon_material _weapon_mesh) (break `/Game/Data/Structures/laser_params` laser_params))
  (bind _output_get (set `self.base_speed` _base_speed))
  (set `self.base_damage` _base_damage)
  (set `self.base_lifespan` _base_lifespan)
  (set `self.base_scale` _scale)
  (set `self.laser_volume` _weapon_volume)
  (set `self.laser_sound` _weapon_sound)
  (set `self.reload_volume` _reload_volume)
  (set `self.reload_sound` _reload_sound)
  (`PrimitiveComponent.SetMaterial` (`self.Laser`) 0 _weapon_material)
  (`StaticMeshComponent.SetStaticMesh` (`self.Laser`) _weapon_mesh)
  (set `ProjectileMovementComponent.MaxSpeed` _output_get (`self.ProjectileMovement`))
  (return _attenuation _concurrency))

(fn `UserConstructionScript`)