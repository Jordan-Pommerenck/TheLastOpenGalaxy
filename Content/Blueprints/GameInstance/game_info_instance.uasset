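; Game Instance that opens the game's front-end menus: main title screen, settings, single-player and mission creator.
; Each menu has its own event that creates the widget on first use, caches it in a variable and adds it to the viewport.
; Only the main menu event enables the mouse cursor and checks whether a cached widget is already on screen before adding it.
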(event `display-main-menu`
  (bind _returnvalue (`GameplayStatics.GetPlayerController` 0))
  (bind _main_menu_wb (`self.main_menu_WB`))
  ;[0.25 0.25 0.25] Show the {Main Menu / TitleScreen} and Enable Mouse Cursor
  (`/Engine/EditorBlueprintResources/StandardMacros.IsValid` (`self.main_menu_WB`)
    (:`Is Valid`
      (if (not (`Widget.IsInViewport` _main_menu_wb))
        (`UserWidget.AddToViewport` _main_menu_wb 0 :!label _label)
        (set `PlayerController.bShowMouseCursor` true _returnvalue)))
    (:`Is Not Valid`
      (bind _returnvalue_2 (`|CreateWidget` "/Game/Blueprints/UI/MainMenu/main.main_C" _returnvalue))
      (set `self.main_menu_WB` _returnvalue_2)
      (goto _label))))

(event `display-settings-menu`
  ;[0.25 0.25 0.25] Show the Options Menu
  (`/Engine/EditorBlueprintResources/StandardMacros.IsValid` (`self.settings_menu_WB`)
    (:`Is Valid`
      _)
    (:`Is Not Valid`
      (bind _returnvalue (`|CreateWidget` "/Game/Blueprints/UI/MainMenu/settings.settings_C" (`GameplayStatics.GetPlayerController` 0)))
      (set `self.settings_menu_WB` _returnvalue)))
  (`UserWidget.AddToViewport` (`self.settings_menu_WB`) 0))

(event `display-single-player-menu`
  ;[0.25 0.25 0.25] Show the Single-Player Menu
  (`/Engine/EditorBlueprintResources/StandardMacros.IsValid` (`self.single_player_WB`)
    (:`Is Valid`
      _)
    (:`Is Not Valid`
      (bind _returnvalue (`|CreateWidget` "/Game/Blueprints/UI/MainMenu/single-player.single-player_C" (`GameplayStatics.GetPlayerController` 0)))
      (set `self.single_player_WB` _returnvalue)))
  (`UserWidget.AddToViewport` (`self.single_player_WB`) 0))

(event `display-mission-creator`
  ;[0.25 0.25 0.25] Show the Single-Player Menu
  (`/Engine/EditorBlueprintResources/StandardMacros.IsValid` (`self.mission_creator_WB`)
    (:`Is Valid`
      _)
    (:`Is Not Valid`
      (bind _returnvalue (`|CreateWidget` "/Game/Blueprints/UI/MainMenu/mission-creator.mission-creator_C" (`GameplayStatics.GetPlayerController` 0)))
      (set `self.mission_creator_WB` _returnvalue)))
  (`UserWidget.AddToViewport` (`self.mission_creator_WB`) 0))