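; Function library of AI helpers for capital ships in a space combat game.
; Simple checks cover disabled systems, team and firing range, while box overlaps gather threats filtered by class and team, and escort allies.
; Threat proximity sets the Fleeing flag, and fighter targeting picks the minimum distance within a scaled laser range, with its line-trace check disconnected.
; Another helper destroys hardpoints with effects and sound.
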(fn `Capital Destroy Hardpoint`
  (params (`Hard-Point` :type "Actor Object Reference") (Sound :type "SoundBase Object Reference") (EmitterTemplate :type "ParticleSystem Object Reference") (`Base-Ship` :type "Object Object Reference") (Scale :type "Float (double-precision)"))
  (`GameplayStatics.SpawnEmitterAtLocation` null EmitterTemplate (.location (`KismetMathLibrary.MakeTransform` (`Actor.K2_GetActorLocation` `Hard-Point`) (`KismetMathLibrary.ComposeRotators` (struct) (struct :`Yaw` 90.0)) (`KismetMathLibrary.Conv_DoubleToVector` Scale))) (.rotation (`KismetMathLibrary.MakeTransform` (`Actor.K2_GetActorLocation` `Hard-Point`) (`KismetMathLibrary.ComposeRotators` (struct) (struct :`Yaw` 90.0)) (`KismetMathLibrary.Conv_DoubleToVector` Scale))) (.scale (`KismetMathLibrary.MakeTransform` (`Actor.K2_GetActorLocation` `Hard-Point`) (`KismetMathLibrary.ComposeRotators` (struct) (struct :`Yaw` 90.0)) (`KismetMathLibrary.Conv_DoubleToVector` Scale))))
  (`GameplayStatics.SpawnSoundAtLocation` null Sound (`Actor.K2_GetActorLocation` `Hard-Point`) (struct) 1.0 1.0 0.0 null null)
  (`Actor.K2_DetachFromActor` `Base-Ship` "KeepRelative" "KeepRelative" "KeepRelative")
  (`KismetArrayLibrary.Array_RemoveItem` (`/Game/Blueprints/AI/AI-CAPITAL-Function-Library.Attached Components` `Base-Ship`) `Hard-Point`)
  (`Actor.K2_DestroyActor` `Hard-Point`)
  (return))

(fn `Capital Find Enemy Threats`
  (params (`Base-Ship` :type "Object Object Reference") (OldNumEnemies :type Integer))
  (returns (`Out Actors` :type "Array of Actor Object Reference") (NewNumEnemies :type Integer))
  (locals (`Enemy Threats` :type "Array of Actor Object Reference"))
  (bind _outactors (`KismetSystemLibrary.BoxOverlapActors` null (`Actor.K2_GetActorLocation` `Base-Ship`) (`KismetMathLibrary.Conv_DoubleToVector` (`/Game/Blueprints/AI/AI-CAPITAL-Function-Library.AI Sense Radius` `Base-Ship`)) (`|MakeArray` "ObjectTypeQuery1" :!type "EObjectTypeQuery Enum") null (`|MakeArray` null :!type "Actor Object Reference")))
  (bind _returnvalue (`KismetArrayLibrary.Array_Length` _outactors))
  (if (== _returnvalue OldNumEnemies)
    (bind _output_get (set `local.Enemy Threats` _outactors))
    (for _array_element _output_get
      (bind _ashuman_fighter (cast `` _array_element))
      (if (and (<= (`/Game/Blueprints/AI/AI-CAPITAL-Function-Library.AICapitalClass` _ashuman_fighter) (`/Game/Blueprints/AI/AI-CAPITAL-Function-Library.AICapitalClass` `Base-Ship`)) (!= (`/Game/Blueprints/AI/AI-CAPITAL-Function-Library.Human Team` _ashuman_fighter) (`/Game/Blueprints/AI/AI-CAPITAL-Function-Library.Human Team` `Base-Ship`)))
        (`KismetArrayLibrary.Array_RemoveItem` (`local.Enemy Threats`) _ashuman_fighter))))
  (return (`local.Enemy Threats`) _returnvalue))

(fn `Capital Find Escort Ally`
  (params (`Base-Ship` :type "Object Object Reference"))
  (returns (`Escort Ally` :type "Object Object Reference"))
  (locals (`Escort Allies` :type "Map of Object Object Reference to Float (double-precision)"))
  (bind (_escort_allies _escort_allies_2) (`local.Escort Allies`))
  (bind _outactors (`KismetSystemLibrary.BoxOverlapActors` null (`Actor.K2_GetActorLocation` `Base-Ship`) (`KismetMathLibrary.Conv_DoubleToVector` (`/Game/Blueprints/AI/AI-CAPITAL-Function-Library.AI Sense Radius` `Base-Ship`)) (`|MakeArray` "ObjectTypeQuery1" :!type "EObjectTypeQuery Enum") null (`|MakeArray` null :!type "Actor Object Reference")))
  (if (> (`KismetArrayLibrary.Array_Length` _outactors) 0)
    (for _array_element _outactors
      (bind _ashuman_fighter (cast `` _array_element))
      (if (`|EnumEquality` _)
        (`BlueprintMapLibrary.Map_Add` (`.Escort Allies` (`local.Escort Allies`)) _ashuman_fighter (`Actor.GetDistanceTo` _ashuman_fighter null))))
    (bind _values (`BlueprintMapLibrary.Map_Values` _escort_allies_2))
    (bind _keys (`BlueprintMapLibrary.Map_Keys` _escort_allies_2))
    (return (`|GetArrayItem` _keys (`KismetMathLibrary.MinOfFloatArray` _values)))))

(fn `Capital Find Nearest Fighter`
  (params (`Base-Ship` :type "Object Object Reference") (LASER :type "Actor Object Reference") (`Laser Component Spawn` :type "SceneComponent Object Reference") (`Laser Range` :type "Float (double-precision)"))
  (returns (Output :type "Actor Object Reference"))
  (locals (Distances :type "Array of Float (double-precision)"))
  (bind _fightertargets (`/Game/Blueprints/AI/AI-CAPITAL-Function-Library.FighterTargets` `Base-Ship`))
  (bind _indexofminvalue (`KismetMathLibrary.MinOfFloatArray` (`local.Distances`)))
  (bind _output (`|GetArrayItem` _fightertargets _indexofminvalue))
  (for _array_element _fightertargets
    (`/Engine/EditorBlueprintResources/StandardMacros.IsValid` _array_element
      (:`Is Valid`
        (bind _returnvalue (`Actor.GetDistanceTo` `Base-Ship` _array_element))
        (if (and true (<= _returnvalue (* `Laser Range` 14.603174 1000.0)))
          (`KismetArrayLibrary.Array_Add` (`local.Distances`) _returnvalue)))))
  (if (>= _indexofminvalue 0)
    (`/Engine/EditorBlueprintResources/StandardMacros.IsValid` _output
      (:`Is Valid`
        (return _output)))))

(fn `Capital Flee Enemies in Threat Distance`
  (params (`Enemy Threats` :type "Array of Actor Object Reference") (`Base-Ship` :type "Object Object Reference"))
  (returns (Fleeing :type Boolean) (`Distance to Target` :type "Float (double-precision)") (`Threat Distance` :type "Float (double-precision)") (MyTarget :type "Object Object Reference"))
  (bind _threat_distance (`/Game/Blueprints/AI/AI-CAPITAL-Function-Library.Threat Distance` `Base-Ship`))
  (`/Engine/EditorBlueprintResources/StandardMacros.IsValid` `Base-Ship`
    (:`Is Valid`
      (for _array_element `Enemy Threats`
        (`/Engine/EditorBlueprintResources/StandardMacros.IsValid` _array_element
          (:`Is Valid`
            (bind _ashuman_fighter (cast `` _array_element))
            (bind _returnvalue (`Actor.GetDistanceTo` _ashuman_fighter `Base-Ship`))
            (if (< _returnvalue _threat_distance)
              (set `/Game/Blueprints/AI/AI-CAPITAL-Function-Library.Fleeing` true `Base-Ship`)
              (else
                (set `/Game/Blueprints/AI/AI-CAPITAL-Function-Library.Fleeing` false `Base-Ship`))))))
      (`/Engine/EditorBlueprintResources/StandardMacros.IsValid` _ashuman_fighter
        (:`Is Valid`
          (return (`/Game/Blueprints/AI/AI-CAPITAL-Function-Library.Fleeing` `Base-Ship`) _returnvalue _threat_distance _ashuman_fighter))))))

(fn `Capital I am Disabled`
  (params (Target :type "Object Object Reference") (`Fraction Disabled` :type "Float (double-precision)"))
  (returns (`Return Value` :type Boolean))
  (return (< (`/Game/Blueprints/AI/AI-CAPITAL-Function-Library.Systems` Target) (`KismetMathLibrary.FTrunc` (* (`/Game/Blueprints/AI/AI-CAPITAL-Function-Library.BaseSystems` Target) `Fraction Disabled`)))))

(fn `Capital Laser Line Trace`
  (params (`AI-Capital Target` :type "Actor Object Reference") (`Laser Component Spawn` :type "SceneComponent Object Reference") (WeaponSelf :type "Actor Object Reference"))
  (returns (OutHit :type "HitResult Structure") (HitActor :type "Actor Object Reference"))
  (bind _returnvalue (`SceneComponent.K2_GetComponentLocation` `Laser Component Spawn`))
  (bind _outhit (`KismetSystemLibrary.SphereTraceSingleForObjects` null _returnvalue (+ _returnvalue (* (`Actor.K2_GetActorLocation` `AI-Capital Target`) (* (`Actor.GetDistanceTo` `AI-Capital Target` WeaponSelf) 2.0))) 20.0 (`|MakeArray` "ObjectTypeQuery1" :!type "EObjectTypeQuery Enum") true (`|MakeArray` WeaponSelf) "Persistent"))
  (return _outhit (`.HitActor` (`GameplayStatics.BreakHitResult` _outhit))))

(fn `Capital Target Distance`
  (params (`Base-Ship` :type "Object Object Reference"))
  (returns (`Return Value` :type Boolean) (Distance :type "Float (double-precision)"))
  (bind _returnvalue (`Actor.GetDistanceTo` `Base-Ship` (`/Game/Blueprints/AI/AI-CAPITAL-Function-Library.MyTarget` `Base-Ship`)))
  (return (< _returnvalue (`/Game/Blueprints/AI/AI-CAPITAL-Function-Library.FiringRange` `Base-Ship`)) _returnvalue))

(fn `Capital Target on Same Team`
  (params (Target :type "Object Object Reference") (`AI-Capital` :type "Object Object Reference"))
  (returns (`Return Value` :type Boolean))
  (return (== (`/Game/Blueprints/AI/AI-CAPITAL-Function-Library.My Team` Target) (`/Game/Blueprints/AI/AI-CAPITAL-Function-Library.My Team` `AI-Capital`))))